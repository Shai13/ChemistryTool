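; AtomBP is a clickable atom actor that pairs with another atom through two successive clicks.
; The first click stores the actor as LastClicked on MyGameInstance, which acts as shared selection state between atoms.
; The next click saves that stored actor in the clicked atom's Bond variable and clears the selection, so the link is one-way.
; Print strings trace each click, and the T key prints a test message.
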(event `self.ReceiveActorOnClicked`
  (`KismetSystemLibrary.PrintString` "click")
  (bind _asmy_game_instance (cast `/Game/Blueprints/MyGameInstance` (`GameplayStatics.GetGameInstance`)))
  (bind _lastclicked (`/Game/Blueprints/MyGameInstance.LastClicked` _asmy_game_instance))
  (if (`KismetSystemLibrary.IsValid` _lastclicked)
    (set `self.Bond` _lastclicked)
    (set `/Game/Blueprints/MyGameInstance.LastClicked` null _asmy_game_instance)
    (`KismetSystemLibrary.PrintString` "bonded")
    (else
      (set `/Game/Blueprints/MyGameInstance.LastClicked` self _asmy_game_instance)
      (`KismetSystemLibrary.PrintString` "almost bonded"))))

(event `Key|T`
  (:`Pressed`
    (`KismetSystemLibrary.PrintString` "Hello")))

(event `self.ReceiveBeginPlay`)

(event `self.ReceiveActorBeginOverlap`
  (params (OtherActor :type "Actor Object Reference")))

(event `self.ReceiveTick`
  (params (DeltaSeconds :type "Float (single-precision)")))

(fn `UserConstructionScript`)